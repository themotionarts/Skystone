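; Tutorial tip actor that shows a documentation widget when the player enters its trigger, intended for first-time play.
; On BeginPlay it loads the save through MyGameInstance and destroys itself unless the FirstTime flag is set.
; Trigger overlap creates the Widget class on screen if the first found FirstTip widget is not in the viewport.
; Leaving the trigger destroys the actor once that widget exists, without removing the widget.
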(event OnComponentBeginOverlap(Trigger)
  (params (OverlappedComponent :type Primitive%20Component%20Object%20Reference) (OtherActor :type Actor%20Object%20Reference) (OtherComp :type Primitive%20Component%20Object%20Reference) (OtherBodyIndex :type Integer) (bFromSweep :type Boolean) (SweepResult :type Hit%20Result%20Structure%20%28by%20ref%29))
  (if (== OtherActor (Game|GetPlayerCharacter 0))
    (bind _foundwidgets (Widget|GetAllWidgetsOfClass "/Game/UI/Tips/FirstTip.FirstTip_C" true))
    (if (not (UserInterface|Viewport|IsinViewport (Utilities|Array|Get(acopy) _foundwidgets)))
      (bind _returnvalue (UserInterface|CreateWidget (Variables|Default|Getwidget)))
      (UserInterface|Viewport|AddtoViewport _returnvalue 0))))

(event OnComponentEndOverlap(Trigger)
  (params (OverlappedComponent :type Primitive%20Component%20Object%20Reference) (OtherActor :type Actor%20Object%20Reference) (OtherComp :type Primitive%20Component%20Object%20Reference) (OtherBodyIndex :type Integer))
  (if (== OtherActor (Game|GetPlayerCharacter 0))
    (Utilities|IsValid (stale OnComponentBeginOverlap(Trigger) _returnvalue)
      (:Is%20Valid
        (Actor|DestroyActor)))))

(event EventBeginPlay
  (bind _returnvalue (Game|GetGameInstance))
  (bind _asmy_game_instance (Utilities|Casting|CastToMyGameInstance _returnvalue))
  (bind _savegameobject (Variables|/Game/Blueprints/MyGameInstance.MyGameInstance_C|GetSaveGameObject _asmy_game_instance))
  (Default|Load _asmy_game_instance)
  (Variables|Default|SetSAveGameObj _savegameobject)
  (if (not (Variables|/Game/Blueprints/SaveGameObj.SaveGameObj_C|GetFirstTime? _savegameobject))
    (Actor|DestroyActor)))

(event EventTick
  (params (DeltaSeconds :type Float%20%28single-precision%29)))

(fn ConstructionScript)