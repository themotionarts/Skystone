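; AI builder character that hauls bricks to build sites and scores for the Blue Alliance, running at half time dilation.
; Delayed Tick logic moves it to a Brick_Blueprint2, then the nearest Brick_Blueprint1 site.
; It usually replaces the site with Brick_Blueprint3, stacking another site above up to a height limit, but occasionally drops a physics brick.
; FindActorBP measures each brick against itself, so pickup choice ignores proximity.
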(event Custom|FindActorBP
  (bind _outactors (Actor|GetAllActorsOfClass "/Game/Blueprints/Brick_Blueprint2.Brick_Blueprint2_C"))
  (for _array_element _outactors
    (if (not (== (Utilities|GetClass _array_element) "/Game/Blueprints/Brick_Blueprint1.Brick_Blueprint1_C"))
      (if (< (Math|Vector|Distance(Vector) (.location (Transformation|GetActorTransform _array_element)) (.location (Transformation|GetActorTransform _array_element))) (Variables|Default|Getmindist))
        (Variables|Default|Setmindist (Math|Vector|Distance(Vector) (.location (Transformation|GetActorTransform _array_element)) (.location (Transformation|GetActorTransform _array_element))))
        (Variables|Default|Setpos (.location (Transformation|GetActorTransform _array_element)))
        (Variables|Default|SetBrick _array_element))))
  (AI|Navigation|SimpleMovetoActor (Pawn|GetController self) (Variables|Default|GetBrick)))

(event Custom|reset
  (Variables|Default|Setmindist 1e+10)
  (Variables|Default|Setpos "0, 0, 0"))

(event Custom|pick_up_stone
  (Variables|Default|SetFull true)
  (Actor|DestroyActor (Variables|Default|GetBrick))
  (AI|Navigation|SimpleMovetoActor (Pawn|GetController self) (Variables|Default|GetBrick2)))

(event Custom|FindAvailable
  (bind _outactors (Actor|GetAllActorsOfClass "/Game/Blueprints/Brick_Blueprint1.Brick_Blueprint1_C"))
  (for _array_element _outactors
    (if (< (Math|Vector|Distance(Vector) (.location (Transformation|GetActorTransform _array_element)) (.location (Transformation|GetActorTransform))) (Variables|Default|Getmindist2))
      (Variables|Default|Setmindist2 (Math|Vector|Distance(Vector) (.location (Transformation|GetActorTransform _array_element)) (.location (Transformation|GetActorTransform))))
      (Variables|Default|Setpos (.location (Transformation|GetActorTransform _array_element)))
      (Variables|Default|SetBrick2 _array_element))))

(event Custom|ReleaseStone
  (Actor|DestroyActor (Variables|Default|GetBrick2))
  (AI|Navigation|SimpleMovetoActor (Pawn|GetController self) (Variables|Default|GetBrick2)))

(event EventBeginPlay
  (Variables|Default|SetCustomTimeDilation 0.5)
  (CallFunction|FindAvailable)
  (Utilities|FlowControl|Delay 16.0)
  (CallFunction|FindActorBP))

(event EventTick
  (params (DeltaSeconds :type Float%20%28single-precision%29))
  (bind _returnvalue (Game|GetGameInstance))
  (bind _self self)
  (bind _self_2 self)
  (bind _brick2 (Variables|Default|GetBrick2))
  (bind _brick2_2 (Variables|Default|GetBrick2))
  (bind _returnvalue_2 (Pawn|GetController _self_2))
  (bind _returnvalue_3 (Transformation|GetActorLocation _self))
  (bind _asmy_game_instance (Utilities|Casting|CastToMyGameInstance _returnvalue))
  (Utilities|FlowControl|Delay 1.0)
  (Utilities|IsValid (Variables|Default|GetBrick)
    (:Is%20Valid
      (if (< (Math|Vector|Distance(Vector) (Transformation|GetActorLocation (Variables|Default|GetBrick)) _returnvalue_3) 1.3e+02)
        (CallFunction|PickUpStone)
        (CallFunction|FindAvailable)
        (Variables|Default|Setmindist2 1e+09)
        (else
          (AI|Navigation|SimpleMovetoActor _returnvalue_2 (Variables|Default|GetBrick)))))
    (:Is%20Not%20Valid
      (if (Variables|Default|GetFull)
        (Utilities|IsValid (Variables|Default|GetBrick2)
          (:Is%20Valid
            (if (Math|Vector|Equal(Vector) _returnvalue_3 (Transformation|GetActorLocation (Variables|Default|GetBrick2)) 3e+02)
              (if (Math|Boolean|ORBoolean (Math|Random|RandomBool) (Math|Random|RandomBool) (Math|Random|RandomBool) (Math|Random|RandomBool))
                (Variables|Default|SetTransformOfBuilding%20site (Transformation|GetActorTransform _brick2_2))
                (Utilities|IsValid _brick2_2
                  (:Is%20Valid
                    (Actor|DestroyActor _brick2_2)
                    (Game|SpawnActorfromClass "/Game/Blueprints/Brick_Blueprint3.Brick_Blueprint3_C" (Math|Transform|MakeTransform (.location (Variables|Default|GetTransformOfBuilding%20site)) (.rotation (Variables|Default|GetTransformOfBuilding%20site)) "1,1,1") "Undefined" 0 0)
                    (if (<= (.Z (Math|Vector|BreakVector (.location (Variables|Default|GetTransformOfBuilding%20site)))) 2.3e+02)
                      (Game|SpawnActorfromClass "/Game/Blueprints/Brick_Blueprint1.Brick_Blueprint1_C" (Math|Transform|MakeTransform (Math|Vector|MakeVector (.X (Math|Vector|BreakVector (.location (Variables|Default|GetTransformOfBuilding%20site)))) (.Y (Math|Vector|BreakVector (.location (Variables|Default|GetTransformOfBuilding%20site)))) (+ (.Z (Math|Vector|BreakVector (.location (Variables|Default|GetTransformOfBuilding%20site)))) 25.0)) (.rotation (Variables|Default|GetTransformOfBuilding%20site)) "1,1,1") "Undefined" 0 0))
                    (Variables|Default|SetFull false)
                    (Variables|/Game/Blueprints/MyGameInstance.MyGameInstance_C|SetScoreBlueAlliance _asmy_game_instance (+ (Variables|/Game/Blueprints/MyGameInstance.MyGameInstance_C|GetScoreBlueAlliance _asmy_game_instance) 5))
                    (CallFunction|FindAvailable))
                  (:Is%20Not%20Valid
                    (CallFunction|FindAvailable)))
                (else
                  (bind _returnvalue_4 (Game|SpawnActorfromClass "/Game/Blueprints/Brick_Blueprint3.Brick_Blueprint3_C" (Math|Transform|MakeTransform (+ (Transformation|GetActorLocation self) "0,40.000000,0.000000") "30.000000,30.000000, 0" "1,1,1") "Undefined" 0 0))
                  (Physics|SetSimulatePhysics (Variables|/Script/Engine.StaticMeshActor|GetStaticMeshComponent _returnvalue_4) true)
                  (Variables|Default|SetFull false)
                  (CallFunction|FindAvailable)))
              (else
                (Utilities|IsValid _brick2
                  (:Is%20Valid
                    _)
                  (:Is%20Not%20Valid
                    (CallFunction|FindAvailable)))
                (AI|Navigation|SimpleMovetoActor _returnvalue_2 _brick2))))
          (:Is%20Not%20Valid
            (CallFunction|FindAvailable)))
        (else
          (CallFunction|Reset)
          (CallFunction|FindActorBP))))))

(fn ConstructionScript)