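; HumanPlayer is a Blueprint that keeps a brick present in the level.
; On BeginPlay and every Tick, Check searches for all Brick_Blueprint actors and caches the first as Brick.
; When that reference is invalid, Tick runs two spawns at fixed locations: one with no class specified, then a new Brick_Blueprint.
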(event Custom|Check
  (bind _outactors (Actor|GetAllActorsOfClass "/Game/Blueprints/Brick_Blueprint.Brick_Blueprint_C"))
  (Variables|Default|SetBrick (Utilities|Array|Get(acopy) _outactors)))

(event EventBeginPlay
  (CallFunction|Check))

(event EventTick
  (params (DeltaSeconds :type Float%20%28single-precision%29))
  (CallFunction|Check)
  (Utilities|IsValid (Variables|Default|GetBrick)
    (:Is%20Not%20Valid
      (Game|SpawnActorfromClass "/Game/Blueprints/Brick_Blueprint.Brick_Blueprint_C" (Math|Transform|MakeTransform "26.000000,-268.000000,130.000000" "0, 0, 0" "1,1,1") "Undefined" 0 0)
      (Game|SpawnActorfromClass "/Game/Blueprints/Brick_Blueprint.Brick_Blueprint_C" (Math|Transform|MakeTransform "-60.000000,450.000000,231.000000" "0, 0, 0" "1,1,1") "Undefined" 0 0))))

(fn ConstructionScript)