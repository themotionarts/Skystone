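; Enemy AI character that collects bricks and delivers them to a drop-off point, starting after a delay at half time dilation.
; FindActorBP picks the nearest BrickClass2 actor, and a Delay-throttled Tick walks to it with simple move nodes.
; Pickup destroys the brick and marks the character Full.
; At Loc it spawns a BrickClass actor at SpawnLoc, disables stepping up on it, then searches again.
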(event Custom|FindActorBP
  (bind _outactors (Actor|GetAllActorsOfClass (Variables|Default|GetBrickClass2)))
  (for _array_element _outactors
    (if (< (Math|Vector|Distance(Vector) (.location (Transformation|GetActorTransform _array_element)) (.location (Transformation|GetActorTransform))) (Variables|Default|Getmindist))
      (Variables|Default|Setmindist (Math|Vector|Distance(Vector) (.location (Transformation|GetActorTransform _array_element)) (.location (Transformation|GetActorTransform))))
      (Variables|Default|SetBrick _array_element))))

(event Custom|reset
  (Variables|Default|Setmindist 1e+10))

(event Custom|pick_up_stone
  (Variables|Default|SetFull true)
  (Actor|DestroyActor (Variables|Default|GetBrick))
  (AI|Navigation|SimpleMovetoLocation (Pawn|GetController self) (Variables|Default|GetLoc)))

(event EventBeginPlay
  (Utilities|FlowControl|Delay 6.0)
  (CallFunction|FindActorBP)
  (Variables|Default|SetCanplay true)
  (Variables|Default|SetCustomTimeDilation 0.5))

(event EventTick
  (params (DeltaSeconds :type Float%20%28single-precision%29))
  (bind _self self)
  (bind _loc (Variables|Default|GetLoc))
  (bind _returnvalue (Transformation|GetActorLocation _self))
  (if (Variables|Default|GetCanplay)
    (Utilities|FlowControl|Delay 1.0)
    (Utilities|IsValid (Variables|Default|GetBrick)
      (:Is%20Valid
        (if (< (Math|Vector|Distance(Vector) (Transformation|GetActorLocation (Variables|Default|GetBrick)) _returnvalue) 1.3e+02)
          (CallFunction|PickUpStone)
          (else
            (AI|Navigation|SimpleMovetoActor (Pawn|GetController self) (Variables|Default|GetBrick)))))
      (:Is%20Not%20Valid
        (if (Variables|Default|GetFull)
          (if (Math|Vector|Equal(Vector) _returnvalue (Variables|Default|GetLoc) 1e+02)
            (bind _returnvalue_2 (Game|SpawnActorfromClass (Variables|Default|GetBrickClass) (Math|Transform|MakeTransform (Variables|Default|GetSpawnLoc) "0, 0, 0" "1,1,1") "Undefined" 0 0))
            (Variables|Default|SetFull false)
            (Variables|/Script/Engine.PrimitiveComponent|SetCanCharacterStepUpOn (Actor|GetComponentbyClass _returnvalue_2 "/Script/Engine.StaticMeshComponent") "ECB_No")
            (else
              (AI|Navigation|SimpleMovetoLocation (Pawn|GetController self) (Math|Vector|MakeVector (.x _loc) (.y _loc) (.z _loc)))))
          (else
            (CallFunction|Reset)
            (CallFunction|FindActorBP)))))))

(fn ConstructionScript)