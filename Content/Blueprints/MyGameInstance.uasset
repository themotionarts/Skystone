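; Game instance that loads and saves the SkyStone save slot, which holds crosshair and sound settings.
; Load reads the slot and copies crosshair, master sound, music and surroundings values into instance variables.
; Save shows a Saving widget for three seconds, reloading any existing save or creating one before writing it.
; Save never copies instance variables back into the save object, and a second save chain is unwired.
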(event Custom|Load
  (bind _returnvalue (SaveGame|LoadGamefromSlot "SkyStone"))
  (bind _assave_game_obj (Utilities|Casting|CastToSaveGameObj _returnvalue))
  (bind _output_get (Variables|Default|SetSaveGameObject _assave_game_obj))
  (Variables|Default|Setcrosshair (Variables|/Game/Blueprints/SaveGameObj.SaveGameObj_C|GetCrosshair _output_get))
  (Variables|Default|Setmaster_sound (Variables|/Game/Blueprints/SaveGameObj.SaveGameObj_C|Getmaster_sound (Variables|Default|GetSaveGameObject)))
  (Variables|Default|Setmusic (Variables|/Game/Blueprints/SaveGameObj.SaveGameObj_C|Getmusic (Variables|Default|GetSaveGameObject)))
  (Variables|Default|Setsurroundings (Variables|/Game/Blueprints/SaveGameObj.SaveGameObj_C|Getsurroundings (Variables|Default|GetSaveGameObject))))

(event Custom|Save
  (Utilities|IsValid (Variables|Default|GetSaveWidget)
    (:Is%20Valid
      _)
    (:Is%20Not%20Valid
      (bind _returnvalue (UserInterface|CreateWidget "/Game/UI/Saving.Saving_C"))
      (Variables|Default|SetSaveWidget _returnvalue)))
  (UserInterface|Viewport|AddtoViewport (Variables|Default|GetSaveWidget) 0)
  (bind _returnvalue_2 (SaveGame|DoesSaveGameExist "SkyStone"))
  (if _returnvalue_2
    (CallFunction|Load)
    (else
      (bind _returnvalue_3 (SaveGame|CreateSaveGameObject "/Game/Blueprints/SaveGameObj.SaveGameObj_C"))
      (Variables|Default|SetSaveGameObject _returnvalue_3)))
  (SaveGame|SaveGametoSlot (Variables|Default|GetSaveGameObject) "SkyStone")
  (Utilities|FlowControl|Delay 3.0)
  (Widget|RemovefromParent (Variables|Default|GetSaveWidget)))