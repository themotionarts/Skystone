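; Multiplayer game state that runs the timed round on GameMap using server world time.
; BeginPlay caches the PauseMenu widget and adds a HUD widget on GameMap, or enables character movement immediately on other maps.
; Tick feeds the 126-second countdown to PauseMenu and unlocks movement after five seconds.
; Once time expires, it adds a Loading widget targeting EndGame, repeating every tick without a guard.
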(event EventBeginPlay
  (bind _returnvalue (Game|GetPlayerCharacter 0))
  (bind _foundwidgets (Widget|GetAllWidgetsOfClass "/Game/UI/PauseMenu.PauseMenu_C" true))
  (Variables|Default|SetPause (Utilities|Array|Get(acopy) _foundwidgets))
  (bind _returnvalue_2 (Game|GetCurrentLevelName true))
  (Variables|Default|SetGameMap? (Utilities|Enum|Equal(Enum) _returnvalue_2 "GameMap"))
  (if (Variables|Default|GetGameMap?)
    (bind _returnvalue_3 (UserInterface|CreateWidget (Variables|Default|Getwidget)))
    (UserInterface|Viewport|AddtoViewport _returnvalue_3 0)
    (else
      (Variables|/Game/ThirdPersonCPP/Blueprints/ThirdPersonCharacter.ThirdPersonCharacter_C|SetCanMove_0 (.AsThird%20Person%20Character (Utilities|Casting|CastToThirdPersonCharacter _returnvalue)) true)
      (Variables|/Script/Skystone_working.Skystone_workingCharacter|SetCanMove (.AsSkystone%20Working%20Character (Utilities|Casting|CastToSkystone_workingCharacter _returnvalue)) true))))

(event EventTick
  (params (DeltaSeconds :type Float%20%28single-precision%29))
  (bind _returnvalue (GameState|GetServerWorldTimeSeconds))
  (bind _returnvalue_2 (Game|GetPlayerCharacter 0))
  (bind _returnvalue_3 (- 126.0 _returnvalue))
  (bind _asthird_person_character (Utilities|Casting|CastToThirdPersonCharacter _returnvalue_2))
  (if (Variables|Default|GetGameMap?)
    (Variables|/Game/UI/PauseMenu.PauseMenu_C|SetTime (Variables|Default|GetPause) _returnvalue_3)
    (if (>= _returnvalue_3 0.0)
      (if (>= _returnvalue 5.0)
        (if (not (Variables|/Game/ThirdPersonCPP/Blueprints/ThirdPersonCharacter.ThirdPersonCharacter_C|GetCanMove_0 _asthird_person_character))
          (Variables|/Game/ThirdPersonCPP/Blueprints/ThirdPersonCharacter.ThirdPersonCharacter_C|SetCanMove_0 _asthird_person_character true)
          (Variables|/Script/Skystone_working.Skystone_workingCharacter|SetCanMove (.AsSkystone%20Working%20Character (Utilities|Casting|CastToSkystone_workingCharacter _returnvalue_2)) true)))
      (else
        (bind _returnvalue_4 (UserInterface|CreateWidget "/Game/UI/Loading.Loading_C"))
        (UserInterface|Viewport|AddtoViewport _returnvalue_4 0)
        (Variables|/Game/UI/Loading.Loading_C|SetLevelName _returnvalue_4 "EndGame")))))

(fn ConstructionScript)